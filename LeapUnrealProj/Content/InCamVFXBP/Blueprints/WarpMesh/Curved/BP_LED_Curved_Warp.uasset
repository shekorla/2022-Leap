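; BP_LED_Curved_Warp is a Blueprint that sets up warp meshes for a curved LED screen in an in-camera VFX setup.
; On BeginPlay it calls the warp API to assign four screen mesh components, Screen0 to Screen3, to their matching viewports, vp_0 to vp_3.
; All four assignments share the Root component as origin, and the Tick, overlap and construction script graphs are empty.
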(event `self.ReceiveBeginPlay`
  ;[1 1 1] Setup warp
  (`PicpProjectionBlueprintAPI.AssignWarpMeshToViewport` (`PicpProjectionIBlueprintLib.GetAPI`) "vp_0" (`self.screen_0`) (`self.root`))
  (`PicpProjectionBlueprintAPI.AssignWarpMeshToViewport` (`PicpProjectionIBlueprintLib.GetAPI`) "vp_1" (`self.screen_1`) (`self.root`))
  (`PicpProjectionBlueprintAPI.AssignWarpMeshToViewport` (`PicpProjectionIBlueprintLib.GetAPI`) "vp_2" (`self.screen_2`) (`self.root`))
  (`PicpProjectionBlueprintAPI.AssignWarpMeshToViewport` (`PicpProjectionIBlueprintLib.GetAPI`) "vp_3" (`self.screen_3`) (`self.root`)))

(fn `UserConstructionScript`)